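; Destructible construction light Blueprint with two spot lights that breaks the first time it takes damage.
; On damage, a DoOnce plays a spark sound, activates two spark burst particles and hides both spot lights.
; It also replaces material slot 1 of the mesh with a dynamic instance of Opaque_Inst.
; The construction script creates and stores a dynamic material instance for that same slot.
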(event `self.ReceiveAnyDamage`
  (params (Damage :type "Float (single-precision)") (DamageType :type "DamageType Object Reference") (InstigatedBy :type "Controller Object Reference") (DamageCauser :type "Actor Object Reference"))
  ;[1 1 1] Damage
  (`/Engine/EditorBlueprintResources/StandardMacros.DoOnce` false
    (:`Completed`
      (`AudioComponent.Play` (`self.Reflections_SparkTail_Cue`) 0.0)
      (`ActorComponent.Activate` (`self.P_SparkBurst`) false)
      (`ActorComponent.Activate` (`self.P_SparkBurst_2`) false)
      (`SceneComponent.SetVisibility` (`self.SpotLight`) false false)
      (`SceneComponent.SetVisibility` (`self.SpotLight1`) false false)
      (`PrimitiveComponent.CreateDynamicMaterialInstance` (`self.StaticMesh`) 1 "/Game/RaP_industrial_lights_and_switches/Lights/Materials/Opaque_Inst.Opaque_Inst"))))

(fn `UserConstructionScript`
  (bind _returnvalue (`PrimitiveComponent.CreateDynamicMaterialInstance` (`self.StaticMesh`) 1 null))
  (set `self.Emissive_Brigtness` _returnvalue))